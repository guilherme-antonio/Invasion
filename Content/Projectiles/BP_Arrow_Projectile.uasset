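; BP_Arrow_Projectile is an arrow projectile that damages actors it overlaps and has a limited range.
; On overlap, it skips its owner and applies Damage with the AppliedDamageType_Normal class to actors that have an AC_HealthPoints component, without destroying itself.
; It records its spawn location on BeginPlay, checks the distance from it every Tick, and destroys itself once that reaches MaxRange.
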(event EventBeginPlay
  (bind _output_get (Variables|Default|SetStartLocation (Transformation|GetActorLocation))))

(event Collision|EventActorBeginOverlap
  (params (OtherActor :type Actor%20Object%20Reference))
  (if (!= (Components|GetOwner) OtherActor)
    (Utilities|IsValid (Actor|GetComponentbyClass OtherActor "/Game/Blueprints/ActorCOmponents/HealthSystem/AC_HealthPoints.AC_HealthPoints_C")
      (:Is%20Valid
        (Game|Damage|ApplyDamage OtherActor (Variables|Default|GetDamage) 0 0 "/Game/Blueprints/ActorCOmponents/HealthSystem/AppliedDamageType_Normal.AppliedDamageType_Normal_C")))))

(event EventTick
  (params (DeltaSeconds :type Float%20%28single-precision%29))
  (if (>= (Math|Vector|Distance(Vector) (stale EventBeginPlay _output_get) (Transformation|GetActorLocation)) (Variables|Default|GetMaxRange))
    (Utilities|FlowControl|DoOnce false
      (:Completed
        (Actor|DestroyActor)))))

(fn ConstructionScript)