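; BPC_Ability is an actor component that manages the set of abilities available to its owning pawn.
; It caches the owner as a Pawn on BeginPlay, then InitializeAbilities passes each known class to AddAbilityByClass.
; Each ability is spawned as its own actor, with the pawn as owner and instigator, and stored in AvailableAbilities.
; UseAbility triggers an entry by index through AttemptUseAbility, leaving activation logic to the ability actor.
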(event EventBeginPlay
  (bind _aspawn (Utilities|Casting|CastToPawn (Components|GetOwner)))
  (Variables|Default|SetOwnerPawnRef _aspawn))

(fn AddAbilitybyClass
  (params (AbilityClass :type BP%20Ability%20Class%20Reference))
  (bind _ownerpawnref (Variables|Default|GetOwnerPawnRef))
  (bind _returnvalue (Game|SpawnActorfromClass AbilityClass (Math|Transform|MakeTransform "0, 0, 0" "0, 0, 0" "1.000000,1.000000,1.000000") "Undefined" "MultiplyWithRoot" _ownerpawnref _ownerpawnref))
  (Utilities|Array|Add (Variables|Default|GetAvailableAbilities) _returnvalue)
  (return))

(fn UseAbility
  (params (AbilityIndex :type Integer))
  (Default|AttemptUseAbility (Utilities|Array|Get(acopy) (Variables|Default|GetAvailableAbilities) AbilityIndex))
  (return))

(fn InitializeAbilities
  (params (KnownAbilities :type Array%20of%20BP%20Ability%20Class%20References))
  (for _array_element KnownAbilities
    (CallFunction|AddAbilitybyClass _array_element))
  (return))