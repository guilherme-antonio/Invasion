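; Arrow ability Blueprint for a champion that shows a cursor-aimed targeting indicator; UseAbility is still empty.
; ShowAbilityIndicator calls the parent, then spawns an arrow decal on the champion's capsule if none exists, lowered by the capsule's world height.
; Tick turns the decal toward the point under the cursor and offsets it from the champion along that direction by the indicator size.
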(event EventBeginPlay)

(event Collision|EventActorBeginOverlap
  (params (OtherActor :type Actor%20Object%20Reference)))

(event EventUseAbility)

(event EventShowAbilityIndicator
  (params (Owner :type BP%20Champion%20Object%20Reference))
  (bind _capsulecomponent (Variables|/Script/Engine.Character|GetCapsuleComponent Owner))
  (|CallParentFunction Owner)
  (Utilities|IsValid (Variables|Default|GetAbilityIndicator)
    (:Is%20Not%20Valid
      (Variables|Default|SetChampion Owner)
      (bind _returnvalue (Class|GameplayStatics|SpawnDecalAttached "/Game/Materials/M_ArrowIndicator.M_ArrowIndicator" (Variables|Default|GetIndicatorSize) _capsulecomponent "None" (Math|Vector|MakeVector 0.0 0.0 (* (.z (Transformation|GetWorldLocation _capsulecomponent)) -1.0)) "-90.000000,0.000000,0.000000" "KeepRelativeOffset" 0.0))
      (Variables|Default|SetAbilityIndicator _returnvalue))))

(event EventTick
  (params (DeltaSeconds :type Float%20%28single-precision%29))
  (bind _returnvalue (Game|GetPlayerController 0))
  (bind _indicatorsize (Variables|Default|GetIndicatorSize))
  (bind _champion (Variables|Default|GetChampion))
  (bind _champion_2 (Variables|Default|GetChampion))
  (bind _hitresult (Game|Player|GetHitResultUnderCursorbyChannel _returnvalue "TraceTypeQuery1" true))
  (bind _returnvalue_2 (Transformation|GetActorLocation _champion_2))
  (bind _z (Math|Vector|BreakVector _indicatorsize))
  (bind _capsulecomponent (Variables|/Script/Engine.Character|GetCapsuleComponent _champion))
  (bind _returnvalue_3 (Math|Rotator|FindLookatRotation _returnvalue_2 (.location _hitresult)))
  (bind _returnvalue_4 (Transformation|GetWorldLocation _capsulecomponent))
  (bind _returnvalue_5 (Math|Vector|GetForwardVector (Math|Rotator|MakeRotator (.roll _returnvalue_3) (.pitch _returnvalue_3) (.yaw _returnvalue_3))))
  (Utilities|IsValid (Variables|Default|GetAbilityIndicator)
    (:Is%20Valid
      (if true
        (Transformation|SetWorldLocationAndRotation (Variables|Default|GetAbilityIndicator) (Math|Vector|MakeVector (+ (.x _returnvalue_4) (* (.x _returnvalue_5) _z)) (+ (.y _returnvalue_4) (* (.y _returnvalue_5) _z)) (.z (Transformation|GetWorldLocation (Variables|Default|GetAbilityIndicator)))) (Math|Rotator|MakeRotator 0.0 -9e+01 (.yaw _returnvalue_3)) false false)))))

(fn ConstructionScript
  (|CallParentFunction))