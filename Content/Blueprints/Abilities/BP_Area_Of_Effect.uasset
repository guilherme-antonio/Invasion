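; Area-of-effect ability Blueprint that shows a range decal around the champion and a cursor-driven target area decal.
; ShowAbilityIndicator stores the owner and attaches the range decal to its capsule at a Z offset.
; While that decal exists, Tick spawns the area decal and moves it to the cursor trace hit, clamping X/Y to the range radius along the look-at direction.
; When the range decal is gone, Tick destroys the area decal.
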(event EventBeginPlay)

(event Collision|EventActorBeginOverlap
  (params (OtherActor :type Actor%20Object%20Reference)))

(event EventTick
  (params (DeltaSeconds :type Float%20%28single-precision%29))
  (bind _returnvalue (Game|GetPlayerController 0))
  (bind _champion (Variables|Default|GetChampion))
  (bind _indicatorsize (Variables|Default|GetIndicatorSize))
  (bind _champion_2 (Variables|Default|GetChampion))
  (bind _returnvalue_2 (Transformation|GetActorLocation _champion_2))
  (bind _hitresult (Game|Player|GetHitResultUnderCursorbyChannel _returnvalue "TraceTypeQuery3" true))
  (bind _rootcomponent (Variables|/Script/Engine.Actor|GetRootComponent _champion))
  (bind _returnvalue_3 (Transformation|GetWorldLocation _rootcomponent))
  (bind _returnvalue_4 (Math|Rotator|FindLookatRotation _returnvalue_3 (.location _hitresult)))
  (bind _returnvalue_5 (Math|Vector|GetForwardVector _returnvalue_4))
  (bind _returnvalue_6 (Math|Vector|Normalize _returnvalue_5))
  (Utilities|IsValid (Variables|Default|GetAbilityIndicator)
    (:Is%20Valid
      (Utilities|IsValid (Variables|Default|GetAreaIndicator)
        (:Is%20Valid
          (if (> (Math|Vector|Distance(Vector) (.location _hitresult) (Transformation|GetActorLocation (Variables|Default|GetChampion))) (.z (Variables|Default|GetIndicatorSize)))
            (Transformation|SetWorldLocation (Variables|Default|GetAreaIndicator) (Math|Vector|MakeVector (+ (.x _returnvalue_2) (* (.x _returnvalue_6) (.z _indicatorsize))) (+ (.y _returnvalue_2) (* (.y _returnvalue_6) (.z _indicatorsize))) 0.0) false false)
            (else
              (Transformation|SetWorldLocation (Variables|Default|GetAreaIndicator) (.location _hitresult) false false))))
        (:Is%20Not%20Valid
          (bind _returnvalue_7 (Rendering|Decal|SpawnDecalatLocation "/Game/Materials/M_AOE.M_AOE" (Variables|Default|GetAreaIndicatorSize) (.location _hitresult) "-90.000000,0.000000,0.000000" 0.0))
          (Variables|Default|SetAreaIndicator _returnvalue_7))))
    (:Is%20Not%20Valid
      (Utilities|IsValid (Variables|Default|GetAreaIndicator)
        (:Is%20Valid
          (Components|DestroyComponent (Variables|Default|GetAreaIndicator)))))))

(event EventShowAbilityIndicator
  (params (Owner :type BP%20Champion%20Object%20Reference))
  (bind _capsulecomponent (Variables|/Script/Engine.Character|GetCapsuleComponent Owner))
  (|CallParentFunction Owner)
  (Utilities|IsValid (Variables|Default|GetAbilityIndicator)
    (:Is%20Not%20Valid
      (Variables|Default|SetChampion Owner)
      (bind _returnvalue (Class|GameplayStatics|SpawnDecalAttached "/Game/Materials/M_Indicator.M_Indicator" (Variables|Default|GetIndicatorSize) _capsulecomponent "None" (Math|Vector|MakeVector 0.0 0.0 (* (.z (Transformation|GetWorldLocation _capsulecomponent)) -1.0)) "-90.000000,0.000000,0.000000" "KeepRelativeOffset" 0.0))
      (Variables|Default|SetAbilityIndicator _returnvalue))))

(fn ConstructionScript
  (|CallParentFunction))