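; Damage zone actor that applies damage to a BP_Champion while it overlaps the box.
; BeginPlay creates a damage timer and pauses it immediately.
; A champion entering the box is stored and unpauses the timer, whose event damages that stored champion.
; Any end overlap pauses the timer, regardless of which actor leaves.
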(event OnComponentBeginOverlap(Box)
  (params (OverlappedComponent :type Primitive%20Component%20Object%20Reference) (OtherActor :type Actor%20Object%20Reference) (OtherComp :type Primitive%20Component%20Object%20Reference) (OtherBodyIndex :type Integer) (bFromSweep :type Boolean) (SweepResult :type Hit%20Result%20Structure%20%28by%20ref%29))
  (bind _asbp_champion (Utilities|Casting|CastToBP_Champion OtherActor))
  (Variables|Default|SetChampion _asbp_champion)
  (Utilities|Time|UnpauseTimerbyHandle (Variables|Default|GetDamageTimer)))

(event OnComponentEndOverlap(Box)
  (params (OverlappedComponent :type Primitive%20Component%20Object%20Reference) (OtherActor :type Actor%20Object%20Reference) (OtherComp :type Primitive%20Component%20Object%20Reference) (OtherBodyIndex :type Integer))
  (Utilities|Time|PauseTimerbyHandle (Variables|Default|GetDamageTimer)))

(event Custom|CauseDamage
  (bind _champion (Variables|Default|GetChampion))
  (Utilities|IsValid _champion
    (:Is%20Valid
      (Game|Damage|ApplyDamage _champion 0.0 0 0))))

(event EventBeginPlay
  (bind _returnvalue (Utilities|Time|SetTimerbyEvent (delegate Custom|CauseDamage) 0.0))
  (bind _output_get (Variables|Default|SetDamageTimer _returnvalue))
  (Utilities|Time|PauseTimerbyHandle _output_get))

(fn ConstructionScript)