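; Actor component that gives its owner hit points with damage resistance and timed regeneration, destroying the owner when damage depletes them.
; TakeDamage fires a dispatcher, then ApplyResistance casts the damage type to AppliedDamageType, reducing Normal damage by a resistance percentage while True damage passes unchanged.
; A looping timer calls RegenerateHP, which fires its own dispatcher, pauses at max HP and is resumed by non-lethal damage.
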(event EventBeginPlay
  (Variables|Default|SetCurrentHP (Variables|Default|GetMaxHP))
  (bind _returnvalue (Utilities|Time|SetTimerbyFunctionName 0 "RegenerateHP" (Variables|Default|GetHPRegenerationRate) true))
  (Variables|Default|SetRegenerationTimeHandler _returnvalue))

(fn ApplyResistance
  (params (DamageAmount :type Float%20%28double-precision%29) (DamageType :type Damage%20Type%20Object%20Reference))
  (bind _asapplied_damage_type (Utilities|Casting|CastToAppliedDamageType DamageType))
  (bind _edamagetype (Default|GetEDamageType _asapplied_damage_type))
  (switch Utilities|FlowControl|Switch|SwitchonEDamageType _edamagetype
    (:NewEnumerator0
      (LocalVariables|SetCalculatedDamage DamageAmount))
    (:NewEnumerator1
      (LocalVariables|SetCalculatedDamage (- DamageAmount (* (/ (Variables|Default|GetResistance) 1e+02) DamageAmount)))))
  (return (LocalVariables|GetCalculatedDamage)))

(fn RegenerateHP
  (bind _maxhp (Variables|Default|GetMaxHP))
  (Default|CallOnHealthRegenerated)
  (if (>= (+ (Variables|Default|GetHPRegeneration) (Variables|Default|GetCurrentHP)) _maxhp)
    (Variables|Default|SetCurrentHP _maxhp)
    (Utilities|Time|PauseTimerbyHandle (Variables|Default|GetRegenerationTimeHandler))
    (else
      (Variables|Default|SetCurrentHP (+ (Variables|Default|GetHPRegeneration) (Variables|Default|GetCurrentHP))))))

(fn TakeDamage
  (params (DamageAmount :type Float%20%28double-precision%29) (DamageType :type Damage%20Type%20Object%20Reference))
  (Default|CallOnDamageTaken)
  (bind _returndamage (CallFunction|ApplyResistance DamageAmount DamageType))
  (if (<= (- (Variables|Default|GetCurrentHP) _returndamage) 0.0)
    (Actor|DestroyActor (Components|GetOwner))
    (else
      (Variables|Default|SetCurrentHP (- (Variables|Default|GetCurrentHP) _returndamage))
      (Utilities|Time|UnpauseTimerbyHandle (Variables|Default|GetRegenerationTimeHandler)))))