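; BP_HealthBar is a widget component that displays a health bar driven by a health point component.
; SetEvents stores the supplied health point component and binds to its damage-taken and health-regenerated events.
; HealthChanged sets the HealthBar percent in WE_CharacterWidget to current over max HP, so updates are event-driven rather than polled on Tick.
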(event Custom|HealthChanged
  (bind _healthpointcomponent (Variables|Default|GetHealthPointComponent))
  (bind _aswe_character_widget (Utilities|Casting|CastToWE_CharacterWidget (UserInterface|GetUserWidgetObject)))
  (Variables|/Script/UMG.ProgressBar|SetPercent (Variables|/Game/Blueprints/Widgets/WE_CharacterWidget.WE_CharacterWidget_C|GetHealthBar _aswe_character_widget) (/ (Variables|/Game/Blueprints/ActorCOmponents/HealthSystem/AC_HealthPoints.AC_HealthPoints_C|GetCurrentHP _healthpointcomponent) (Variables|/Game/Blueprints/ActorCOmponents/HealthSystem/AC_HealthPoints.AC_HealthPoints_C|GetMaxHP _healthpointcomponent))))

(event EventTick
  (params (DeltaSeconds :type Float%20%28single-precision%29)))

(fn SetEvents
  (params (NewParam :type AC%20Health%20Points%20Object%20Reference))
  (bind _output_get (Variables|Default|SetHealthPointComponent NewParam))
  (EventDispatchers|BindEventtoOnHealthRegenerated _output_get (EventDispatchers|CreateEvent :!event Custom|HealthChanged))
  (EventDispatchers|BindEventtoOnDamageTaken _output_get (EventDispatchers|CreateEvent :!event Custom|HealthChanged)))