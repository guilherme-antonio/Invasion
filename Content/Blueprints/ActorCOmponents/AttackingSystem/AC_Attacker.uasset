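; AC_Attacker is an actor component that carries out a champion's basic attack on its current target, either ranged or melee.
; AttackTarget checks that the target is valid, then branches on IsRanged.
; Ranged attacks spawn a homing projectile at the owner's "Projectile"-tagged arrow, pass it the attack damage and steer it toward the target's mesh component.
; Melee attacks apply damage to the target immediately with the normal damage type.
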(event EventBeginPlay)

(event EventTick
  (params (DeltaSeconds :type Float%20%28single-precision%29)))

(fn AttackTarget
  (bind _targettoattack (Variables|Default|GetTargetToAttack))
  (Utilities|IsValid _targettoattack
    (:Is%20Valid
      (if (Variables|Default|GetIsRanged)
        (bind _returnvalue (Game|SpawnActorfromClass "/Game/Projectiles/BP_Champion_Attack_Projectile.BP_Champion_Attack_Projectile_C" (Transformation|GetWorldTransform (Utilities|Array|Get(acopy) (Actor|GetComponentsbyTag (Components|GetOwner) "/Script/Engine.ArrowComponent" "Projectile"))) "Undefined" "MultiplyWithRoot" 0 0))
        (Variables|/Game/Projectiles/BP_Projectile_Base.BP_Projectile_Base_C|SetDamage _returnvalue (Variables|Default|GetAttackDamage))
        (Variables|/Script/Engine.ProjectileMovementComponent|SetHomingTargetComponent (Variables|/Game/Projectiles/BP_Projectile_Base.BP_Projectile_Base_C|GetProjectileMovement _returnvalue) (Actor|GetComponentbyClass (Variables|Default|GetTargetToAttack) "/Script/Engine.MeshComponent"))
        (Variables|/Script/Engine.ProjectileMovementComponent|SetbIsHomingProjectile (Variables|/Game/Projectiles/BP_Projectile_Base.BP_Projectile_Base_C|GetProjectileMovement _returnvalue) true)
        (Variables|/Script/Engine.ProjectileMovementComponent|SetHomingAccelerationMagnitude (Variables|/Game/Projectiles/BP_Projectile_Base.BP_Projectile_Base_C|GetProjectileMovement _returnvalue) 3e+03)
        (else
          (Game|Damage|ApplyDamage _targettoattack (Variables|Default|GetAttackDamage) 0 0 "/Game/Blueprints/ActorCOmponents/HealthSystem/AppliedDamageType_Normal.AppliedDamageType_Normal_C"))))))