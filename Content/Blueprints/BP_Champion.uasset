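; BP_Champion is a player-controlled champion with MOBA-style mouse and hotkey controls for moving, attacking and using abilities.
; Right-click moves to the cursor's trace point; left-click fires the ability with an active indicator, otherwise attacks through AC_Attacker.
; A shows an attack-range decal, letting a click on a non-damageable actor target the closest one within range.
; BPCAbility initializes starting abilities, while AC_HealthPoints takes damage and updates the health bar widget.
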(event OnDamageTaken(AC_HealthPoints)
  (bind _ac_healthpoints (Variables|Default|GetAC_HealthPoints))
  (bind _aswe_character_widget (Utilities|Casting|CastToWE_CharacterWidget (UserInterface|GetWidget (Variables|Default|GetHealthBar))))
  (Progress|SetPercent (Variables|/Game/Blueprints/Widgets/WE_CharacterWidget.WE_CharacterWidget_C|GetHealthBar _aswe_character_widget) (/ (Variables|/Game/Blueprints/ActorCOmponents/HealthSystem/AC_HealthPoints.AC_HealthPoints_C|GetCurrentHP _ac_healthpoints) (Variables|/Game/Blueprints/ActorCOmponents/HealthSystem/AC_HealthPoints.AC_HealthPoints_C|GetMaxHP _ac_healthpoints))))

(event OnHealthRegenerated(AC_HealthPoints)
  (bind _ac_healthpoints (Variables|Default|GetAC_HealthPoints))
  (bind _aswe_character_widget (Utilities|Casting|CastToWE_CharacterWidget (UserInterface|GetWidget (Variables|Default|GetHealthBar))))
  (Progress|SetPercent (Variables|/Game/Blueprints/Widgets/WE_CharacterWidget.WE_CharacterWidget_C|GetHealthBar _aswe_character_widget) (/ (Variables|/Game/Blueprints/ActorCOmponents/HealthSystem/AC_HealthPoints.AC_HealthPoints_C|GetCurrentHP _ac_healthpoints) (Variables|/Game/Blueprints/ActorCOmponents/HealthSystem/AC_HealthPoints.AC_HealthPoints_C|GetMaxHP _ac_healthpoints))))

(event EventBeginPlay
  (Default|InitializeAbilities (Variables|Default|GetBPC_Ability) (Variables|Default|GetStartingAbilities)))

(event Game|Damage|EventAnyDamage
  (params (Damage :type Float%20%28single-precision%29) (DamageType :type Damage%20Type%20Object%20Reference) (InstigatedBy :type Controller%20Object%20Reference) (DamageCauser :type Actor%20Object%20Reference))
  (Default|TakeDamage (Variables|Default|GetAC_HealthPoints) Damage DamageType))

(event Input|KeyboardEvents|Q
  (params (Key :type Key%20Structure :default "None"))
  (:Pressed
    (Default|ShowAbilityIndicator (Utilities|Array|Get(acopy) (Variables|/Game/Blueprints/Abilities/BPC_Ability.BPC_Ability_C|GetAvailableAbilities (Variables|Default|GetBPC_Ability))) self)))

(event Input|MouseEvents|RightMouseButton
  (params (Key :type Key%20Structure :default "None"))
  (:Pressed
    (CallFunction|MovetoPosition)))

(event Input|KeyboardEvents|S
  (params (Key :type Key%20Structure :default "None"))
  (:Pressed
    (Components|Movement|StopMovementImmediately (Variables|Character|GetCharacterMovement))))

(event Input|KeyboardEvents|A
  (params (Key :type Key%20Structure :default "None"))
  (:Pressed
    (CallFunction|CreateAttackIndicator)
    (CallFunction|RemoveAbilityIndicator)))

(event Input|MouseEvents|LeftMouseButton
  (params (Key :type Key%20Structure :default "None"))
  (:Pressed
    (bind _ability (CallFunction|CheckAbilityUse))
    (Utilities|IsValid _ability
      (:Is%20Valid
        (Default|AttemptUseAbility _ability))
      (:Is%20Not%20Valid
        (CallFunction|AttackTarget)))))

(fn ConstructionScript)

(fn AttackTarget
  (bind _returnvalue (Game|GetPlayerController 0))
  (bind (_hitresult _returnvalue_2) (Game|Player|GetHitResultUnderCursorbyChannel _returnvalue "TraceTypeQuery1" true))
  (if _returnvalue_2
    (LocalVariables|SetTarget (.HitActor (Collision|BreakHitResult _hitresult)))
    (if (== self (LocalVariables|GetTarget))
      (return)
      (else
        (Utilities|IsValid (Actor|GetComponentbyClass (LocalVariables|GetTarget) "/Game/Blueprints/ActorCOmponents/HealthSystem/AC_HealthPoints.AC_HealthPoints_C")
          (:Is%20Valid
            (bind _inrange (CallFunction|IsTargetinRange (LocalVariables|GetTarget)))
            (if _inrange
              (Transformation|SetActorRotation (Math|Rotator|MakeRotator 0.0 0.0 (.yaw (Math|Rotator|FindLookatRotation (Transformation|GetActorLocation) (Transformation|GetActorLocation (LocalVariables|GetTarget))))) :!label _label)
              (Components|Movement|StopMovementImmediately (Actor|GetComponentbyClass "/Script/Engine.CharacterMovementComponent"))
              (if (Variables|Default|GetIsAttackIndicatorShown)
                (Components|DestroyComponent (Variables|Default|GetAttackIndicator))
                (Variables|Default|SetIsAttackIndicatorShown false))
              (bind _asbp_champion (Utilities|Casting|CastToBP_Champion self))
              (Variables|/Game/Blueprints/ActorCOmponents/AttackingSystem/AC_Attacker.AC_Attacker_C|SetTargetToAttack (Variables|BP_Champion_C|GetAC_Attacker _asbp_champion) (LocalVariables|GetTarget))
              (Default|AttackTarget (Variables|BP_Champion_C|GetAC_Attacker _asbp_champion))
              (Variables|/Game/Blueprints/ActorCOmponents/AttackingSystem/AC_Attacker.AC_Attacker_C|SetTargetToAttack (Variables|BP_Champion_C|GetAC_Attacker _asbp_champion) (LocalVariables|GetTarget))
              (return)))
          (:Is%20Not%20Valid
            (if (Variables|Default|GetIsAttackIndicatorShown)
              (bind _realattackrange (CallFunction|GetRealAttackRange))
              (bind (_outactors _returnvalue_3) (Collision|SphereOverlapActors (Transformation|GetActorLocation) _realattackrange (LocalVariables|GetObjectTypes) 0))
              (LocalVariables|SetClosestTargetDistance (+ _realattackrange 1.0))
              (if _returnvalue_3
                (for _array_element _outactors
                  (Utilities|IsValid (Actor|GetComponentbyClass _array_element "/Game/Blueprints/ActorCOmponents/HealthSystem/AC_HealthPoints.AC_HealthPoints_C")
                    (:Is%20Valid
                      (if (and (!= self _array_element) (< (Transformation|GetDistanceTo _array_element self) (LocalVariables|GetClosestTargetDistance)))
                        (LocalVariables|SetClosestTargetDistance (Transformation|GetDistanceTo _array_element self))
                        (LocalVariables|SetClosestTarget _array_element)))))
                (bind _output_get (LocalVariables|SetTarget (LocalVariables|GetClosestTarget)))
                (Utilities|IsValid _output_get
                  (:Is%20Valid
                    (goto _label)))))))))))

(fn GetRealAttackRange
  (return (+ (Variables|/Script/Engine.CapsuleComponent|GetCapsuleRadius (Variables|Collision|GetCapsuleComponent)) (Variables|/Game/Blueprints/ActorCOmponents/AttackingSystem/AC_Attacker.AC_Attacker_C|GetAttackRange (Actor|GetComponentbyClass "/Game/Blueprints/ActorCOmponents/AttackingSystem/AC_Attacker.AC_Attacker_C")))))

(fn IsTargetinRange
  (params (Target :type Actor%20Object%20Reference))
  (bind _realattackrange (CallFunction|GetRealAttackRange))
  (return (<= (Transformation|GetDistanceTo Target) _realattackrange)))

(fn CreateAttackIndicator
  (bind _returnvalue (Actor|GetComponentbyClass "/Game/Blueprints/ActorCOmponents/AttackingSystem/AC_Attacker.AC_Attacker_C"))
  (bind _capsulecomponent (Variables|Collision|GetCapsuleComponent))
  (bind _attackrange (Variables|/Game/Blueprints/ActorCOmponents/AttackingSystem/AC_Attacker.AC_Attacker_C|GetAttackRange _returnvalue))
  (bind _capsuleradius (Variables|/Script/Engine.CapsuleComponent|GetCapsuleRadius _capsulecomponent))
  (bind _returnvalue_2 (+ _attackrange _capsuleradius))
  (if (not (Variables|Default|GetIsAttackIndicatorShown))
    (bind _returnvalue_3 (Class|GameplayStatics|SpawnDecalAttached "/Game/Materials/M_Indicator.M_Indicator" (Math|Vector|MakeVector 1.0 _returnvalue_2 _returnvalue_2) (Variables|Collision|GetCapsuleComponent) "None" (Math|Vector|MakeVector 0.0 0.0 (* (.z (Transformation|GetWorldLocation _capsulecomponent)) -1.0)) "-90.000000,0.000000,0.000000" "KeepRelativeOffset" 0.0))
    (Variables|Default|SetAttackIndicator _returnvalue_3)
    (Variables|Default|SetIsAttackIndicatorShown true)
    (return)))

(fn MovetoPosition
  (bind _returnvalue (Game|GetPlayerController 0))
  (bind (_worldlocation _worlddirection) (Game|Player|ConvertMouseLocationToWorldSpace _returnvalue))
  (bind _outhit (Collision|LineTraceByChannel _worldlocation (+ _worldlocation (* _worlddirection 1e+04)) "TraceTypeQuery3" false 0 "None"))
  (bind _output_get (Variables|Default|SetLocation (.Location (Collision|BreakHitResult _outhit))))
  (AI|Navigation|SimpleMovetoLocation (Game|GetPlayerController 0) _output_get)
  (Transformation|SetActorRotation (Math|Rotator|MakeRotator 0.0 0.0 (.yaw (Math|Interpolation|RInterpTo (Transformation|GetActorRotation) (Math|Rotator|FindLookatRotation (Transformation|GetActorLocation) _output_get) (Utilities|Time|GetWorldDeltaSeconds) 0.0)))))

(fn CheckAbilityUse
  (bind _array_element (Utilities|Array|ForEachLoopwithBreak (Variables|/Game/Blueprints/Abilities/BPC_Ability.BPC_Ability_C|GetAvailableAbilities (Variables|Default|GetBPC_Ability)) :!label _label)
    (:LoopBody
      (Utilities|IsValid (Variables|/Game/Blueprints/Abilities/BP_Ability.BP_Ability_C|GetAbilityIndicator _array_element)
        (:Is%20Valid
          (LocalVariables|SetCurrentAbility _array_element)
          (goto _label Break))))
    (:Completed
      (return (LocalVariables|GetCurrentAbility)))))

(fn RemoveAbilityIndicator
  (bind _ability (CallFunction|CheckAbilityUse))
  (Utilities|IsValid _ability
    (:Is%20Valid
      (Default|RemoveAbilityIndicator _ability))))

(fn RemoveAttackIndicator
  (if (Variables|Default|GetIsAttackIndicatorShown)
    (Components|DestroyComponent (Variables|Default|GetAttackIndicator))
    (Variables|Default|SetAttackIndicator 0)
    (Variables|Default|SetIsAttackIndicatorShown false)))