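; BP_Camera is a camera actor that becomes the view of the first player controller when play begins.
; Its MoveCamera function pans the actor across the world X and Y axes from two direction inputs, scaled by CameraSpeed and frame delta time.
; Movement uses a world offset without sweeping, so it ignores collision and keeps height constant; the file itself does not call MoveCamera.
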(event EventBeginPlay
  (Game|Player|SetViewTargetwithBlend (Game|GetPlayerController 0) self 0.0 "VTBlend_Linear" 0.0 false))

(event Collision|EventActorBeginOverlap
  (params (OtherActor :type Actor%20Object%20Reference)))

(event EventTick
  (params (DeltaSeconds :type Float%20%28single-precision%29)))

(fn ConstructionScript)

(fn MoveCamera
  (params (XDirection :type Float%20%28double-precision%29) (YDirection :type Float%20%28double-precision%29))
  (Transformation|AddActorWorldOffset (Math|Vector|MakeVector (* (Utilities|Time|GetWorldDeltaSeconds) (* (Variables|Default|GetCameraSpeed) XDirection)) (* (* YDirection (Variables|Default|GetCameraSpeed)) (Utilities|Time|GetWorldDeltaSeconds)) 0.0)))